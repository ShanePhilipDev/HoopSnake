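; BP_Victim is a skeletal-mesh target that gets knocked into ragdoll when the hoop snake character crashes into it.
; Mesh hits from a snake already simulating physics enable physics on a still victim and push it along the reversed hit normal.
; Hits from a snake in hoop mode also force the snake into ragdoll and launch it forward and up.
; Either impact plays a 2D sound once, guarded by a flag.
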(event OnComponentHit(SkeletalMesh)
  (params (HitComponent :type Primitive%20Component%20Object%20Reference) (OtherActor :type Actor%20Object%20Reference) (OtherComp :type Primitive%20Component%20Object%20Reference) (NormalImpulse :type Vector :default "0, 0, 0") (Hit :type Hit%20Result%20Structure%20%28by%20ref%29))
  (bind _bonename (Collision|BreakHitResult Hit))
  (bind _skeletalmesh (Variables|Default|GetSkeletalMesh))
  (bind _skeletalmesh_2 (Variables|Default|GetSkeletalMesh))
  (bind _asbp_hoop_snake_character (Utilities|Casting|CastToBP_HoopSnakeCharacter OtherActor))
  (if (Class|SceneComponent|IsAnySimulatingPhysics (Variables|/Script/Engine.Character|GetMesh _asbp_hoop_snake_character))
    (if (not (Physics|IsSimulatingPhysics _skeletalmesh_2 "None"))
      (Physics|SetSimulatePhysics _skeletalmesh_2 true)
      (Physics|AddImpulse _skeletalmesh_2 (* NormalImpulse -25.0) _bonename false)
      (CallFunction|PlayImpactSound :!label _label))
    (elif (Variables|/Script/HoopSnake.HoopSnakeCharacter|GetbHoopModeEnabled _asbp_hoop_snake_character)
      (Default|ForceRagdoll _asbp_hoop_snake_character)
      (Physics|SetSimulatePhysics _skeletalmesh true)
      (Physics|AddImpulse (Variables|/Script/Engine.Character|GetMesh _asbp_hoop_snake_character) (+ (* (Transformation|GetActorForwardVector _asbp_hoop_snake_character) 2e+02) "0.000000,0.000000,400.000000") "Bone" false)
      (Physics|AddImpulse _skeletalmesh (* NormalImpulse -25.0) _bonename false)
      (goto _label))))

(event EventBeginPlay)

(event Collision|EventActorBeginOverlap
  (params (OtherActor :type Actor%20Object%20Reference)))

(event Collision|EventHit
  (params (MyComp :type Primitive%20Component%20Object%20Reference) (Other :type Actor%20Object%20Reference) (OtherComp :type Primitive%20Component%20Object%20Reference) (bSelfMoved :type Boolean) (HitLocation :type Vector :default "0, 0, 0") (HitNormal :type Vector :default "0, 0, 0") (NormalImpulse :type Vector :default "0, 0, 0") (Hit :type Hit%20Result%20Structure%20%28by%20ref%29)))

(fn ConstructionScript)

(fn PlayImpactSound
  (if (not (Variables|Default|GetSoundPlayed))
    (Variables|Default|SetSoundPlayed true)
    (Audio|PlaySound2D "/Game/HoopSnake/Audio/SC_Impact.SC_Impact" 1.0 1.0 0.0 0 0)))