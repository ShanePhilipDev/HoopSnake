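; BP_Obstacle is a HoopSnake obstacle that knocks the snake character over when it is hit in hoop mode.
; On Hit it casts to BP_HoopSnakeCharacter and acts only if hoop mode is on and the mesh is not already simulating physics.
; It then forces ragdoll, applies a forward and upward impulse to a mesh bone, and plays an impact sound.
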(event EventBeginPlay)

(event Collision|EventActorBeginOverlap
  (params (OtherActor :type Actor%20Object%20Reference)))

(event EventTick
  (params (DeltaSeconds :type Float%20%28single-precision%29)))

(event Collision|EventHit
  (params (MyComp :type Primitive%20Component%20Object%20Reference) (Other :type Actor%20Object%20Reference) (OtherComp :type Primitive%20Component%20Object%20Reference) (bSelfMoved :type Boolean) (HitLocation :type Vector :default "0, 0, 0") (HitNormal :type Vector :default "0, 0, 0") (NormalImpulse :type Vector :default "0, 0, 0") (Hit :type Hit%20Result%20Structure%20%28by%20ref%29))
  (bind _asbp_hoop_snake_character (Utilities|Casting|CastToBP_HoopSnakeCharacter Other))
  (if (not (Class|SceneComponent|IsAnySimulatingPhysics (Variables|/Script/Engine.Character|GetMesh _asbp_hoop_snake_character)))
    (if (Variables|/Script/HoopSnake.HoopSnakeCharacter|GetbHoopModeEnabled _asbp_hoop_snake_character)
      (Default|ForceRagdoll _asbp_hoop_snake_character)
      (Physics|AddImpulse (Variables|/Script/Engine.Character|GetMesh _asbp_hoop_snake_character) (+ (* (Transformation|GetActorForwardVector _asbp_hoop_snake_character) 2e+02) "0.000000,0.000000,400.000000") "Bone" false)
      (Audio|PlaySound2D "/Game/HoopSnake/Audio/SC_Impact.SC_Impact" 1.0 1.0 0.0 0 0))))

(fn ConstructionScript)