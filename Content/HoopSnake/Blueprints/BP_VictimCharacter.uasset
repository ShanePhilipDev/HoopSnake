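; Victim NPC character that shows alert and panic states and gets knocked into a ragdoll by the hoop snake.
; Hide, Alert and Panic events drive a WBP_AlertIcon widget, which Tick yaws toward the camera as a billboard.
; A hit from a ragdolling or hoop-mode snake plays an impact sound and ragdolls the victim, force-ragdolling a hoop-mode snake too.
; Once ragdolled, Tick stops the AI brain logic and hides the icon.
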(event Custom|HideWidget
  (Default|HideAll (Variables|Default|GetAlertWidget)))

(event Custom|Alert
  (bind _alertwidget (Variables|Default|GetAlertWidget))
  (if (not (Widget|IsVisible (Variables|/Game/HoopSnake/UI/WBP_AlertIcon.WBP_AlertIcon_C|GetAlertIcon _alertwidget)))
    (Default|StartAlert _alertwidget)))

(event Custom|Panic
  (bind _alertwidget (Variables|Default|GetAlertWidget))
  (if (not (Widget|IsVisible (Variables|/Game/HoopSnake/UI/WBP_AlertIcon.WBP_AlertIcon_C|GetPanicIcon _alertwidget)))
    (if (Widget|IsVisible (Variables|/Game/HoopSnake/UI/WBP_AlertIcon.WBP_AlertIcon_C|GetAlertIcon (Variables|Default|GetAlertWidget)))
      (Default|AlerttoPanic _alertwidget)
      (else
        (Default|Panic _alertwidget)))))

(event EventBeginPlay
  (bind _aswbp_alert_icon (Utilities|Casting|CastToWBP_AlertIcon (UserInterface|GetUserWidgetObject (Variables|Default|GetAlertIcon))))
  (Variables|Default|SetAlertWidget _aswbp_alert_icon))

(event Collision|EventActorBeginOverlap
  (params (OtherActor :type Actor%20Object%20Reference)))

(event EventTick
  (params (DeltaSeconds :type Float%20%28single-precision%29))
  ;[1 1 1] Billboard widget (always faces camera)
  (Transformation|SetWorldRotation (Variables|Default|GetAlertIcon) (Math|Rotator|MakeRotator 0.0 0.0 (.yaw (Math|Rotator|FindLookatRotation (Transformation|GetWorldLocation (Variables|Default|GetAlertIcon)) (Camera|GetCameraLocation (Game|GetPlayerCameraManager 0))))) false false)
  ;[1 1 1] Stop AI logic and hide widget when ragdolling
  (if (Physics|IsSimulatingPhysics (Variables|Character|GetMesh) "None")
    (bind _asaicontroller (Utilities|Casting|CastToAIController (Pawn|GetController)))
    (AI|Logic|StopLogic (Variables|/Script/AIModule.AIController|GetBrainComponent _asaicontroller) "he dead")
    (Rendering|SetVisibility (Variables|Default|GetAlertIcon) false true)))

(event Collision|EventHit
  (params (MyComp :type Primitive%20Component%20Object%20Reference) (Other :type Actor%20Object%20Reference) (OtherComp :type Primitive%20Component%20Object%20Reference) (bSelfMoved :type Boolean) (HitLocation :type Vector :default "0, 0, 0") (HitNormal :type Vector :default "0, 0, 0") (NormalImpulse :type Vector :default "0, 0, 0") (Hit :type Hit%20Result%20Structure%20%28by%20ref%29))
  ;[1 1 1] When hit by snake, start ragdolling and also force the snake to ragdoll if it is in hoop mode
  (bind _asbp_hoop_snake_character (Utilities|Casting|CastToBP_HoopSnakeCharacter Other))
  (if (Physics|IsSimulatingPhysics (Variables|/Script/Engine.Character|GetMesh _asbp_hoop_snake_character) "None")
    (if (not (Physics|IsSimulatingPhysics (Variables|Character|GetMesh) "None"))
      (Audio|PlaySoundatLocation "/Game/HoopSnake/Audio/SC_Impact.SC_Impact" HitLocation "0, 0, 0" 1.0 1.0 0.0 0 0 0 0 :!label _label)
      (Physics|SetSimulatePhysics (Variables|Character|GetMesh) true))
    (elif (Variables|/Script/HoopSnake.HoopSnakeCharacter|GetbHoopModeEnabled _asbp_hoop_snake_character)
      (Class|HoopSnakeCharacter|ForceRagdoll _asbp_hoop_snake_character)
      (goto _label))))

(fn ConstructionScript)