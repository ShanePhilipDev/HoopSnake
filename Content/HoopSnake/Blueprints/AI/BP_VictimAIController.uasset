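; AI controller for victims in HoopSnake that runs the BT_Victim behavior tree on possession and feeds it sight and hearing perception.
; Sight updates accept only the snake character, setting blackboard sight and snake keys, while hearing records any sensed sound's location.
; Timers delay forgetting: sight's starts when the snake is lost, hearing's restarts with each sound.
; The reset functions clear only the boolean flags, leaving snake and location values in place.
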(event OnTargetPerceptionUpdated(AIPerception)
  (params (Actor :type Actor%20Object%20Reference) (Stimulus :type AI%20Stimulus%20Structure))
  (bind _returnvalue (Class|AIPerceptionSystem|GetSenseClassforStimulus Stimulus))
  (if (== _returnvalue "/Script/AIModule.AISense_Sight")
    (CallFunction|UpdateSight Actor Stimulus)
    (elif (== _returnvalue "/Script/AIModule.AISense_Hearing")
      (CallFunction|UpdateHearing Stimulus))))

(event EventBeginPlay)

(event EventTick
  (params (DeltaSeconds :type Float%20%28single-precision%29)))

(event EventPossess
  (params (PossessedPawn :type Pawn%20Object%20Reference))
  (AI|RunBehaviorTree "/Game/HoopSnake/Blueprints/AI/BT_Victim.BT_Victim"))

(fn ConstructionScript)

(fn UpdateSight
  (params (Actor :type Actor%20Object%20Reference) (Stimulus :type AI%20Stimulus%20Structure))
  (bind _blackboard (Variables|Default|GetBlackboard))
  ;[1 1 1] If can see snake...
  (bind _asbp_hoop_snake_character (Utilities|Casting|CastToBP_HoopSnakeCharacter Actor))
  (if (and (stale _bsuccess) (Utilities|Struct|BreakAIStimulus Stimulus))
    ;[1 1 1] Cancel reset timer and update blackboard values if can see snake
    (Utilities|Time|ClearandInvalidateTimerbyHandle (Variables|Default|GetSightTimerHandle))
    (AI|Components|Blackboard|SetValueasBool _blackboard (Variables|Default|GetSightKey) true)
    (AI|Components|Blackboard|SetValueasObject _blackboard (Variables|Default|GetSnakeKey) _asbp_hoop_snake_character)
    (else
      ;[1 1 1] Begin reset timer if can't see snake
      (bind _returnvalue (Utilities|Time|SetTimerbyEvent (EventDispatchers|CreateEvent :!event ResetSight) (Variables|Default|GetSightResetTime)))
      (Variables|Default|SetSightTimerHandle _returnvalue))))

(fn UpdateHearing
  (params (Stimulus :type AI%20Stimulus%20Structure))
  (bind (_stimuluslocation _bsuccessfullysensed) (Utilities|Struct|BreakAIStimulus Stimulus))
  (bind _blackboard (Variables|Default|GetBlackboard))
  ;[1 1 1] If heard something...
  (if _bsuccessfullysensed
    ;[1 1 1] Cancel reset timer and update blackboard values if can see hear something. Then start reset timer so forget about sound after some time.
    (Utilities|Time|ClearandInvalidateTimerbyHandle (Variables|Default|GetHearingTimerHandle))
    (AI|Components|Blackboard|SetValueasBool _blackboard (Variables|Default|GetHearingKey) true)
    (AI|Components|Blackboard|SetValueasVector _blackboard (Variables|Default|GetSoundLocationKey) _stimuluslocation)
    (bind _returnvalue (Utilities|Time|SetTimerbyEvent (EventDispatchers|CreateEvent :!event ResetHearing) (Variables|Default|GetHearingResetTime)))
    (Variables|Default|SetHearingTimerHandle _returnvalue)))

(fn ResetSight
  (AI|Components|Blackboard|SetValueasBool (Variables|Default|GetBlackboard) (Variables|Default|GetSightKey) false))

(fn ResetHearing
  (AI|Components|Blackboard|SetValueasBool (Variables|Default|GetBlackboard) (Variables|Default|GetHearingKey) false))