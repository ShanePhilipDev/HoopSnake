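; Player controller for Hoop Snake that hides obstacles blocking the camera's view of the snake character.
; Each tick it runs a multi line trace on the Visibility channel from the follow camera to the camera boom and hides the mesh of any BP_Obstacle hit.
; Previously occluded obstacles missing from the current hits are made visible again.
; Visibility toggles instantly, and the occluded list is never pruned.
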(event EventBeginPlay
  (bind _asbp_hoop_snake_character (Utilities|Casting|CastToBP_HoopSnakeCharacter (Game|Player|GetPlayerPawn 0)))
  (Variables|Default|SetSnake _asbp_hoop_snake_character))

(event EventTick
  (params (DeltaSeconds :type Float%20%28single-precision%29))
  (CallFunction|CameraTrace))

(fn ConstructionScript)

(fn CameraTrace
  (bind _snake (Variables|Default|GetSnake))
  ;[1 1 1] Get all objects between camera and focus point, set visibility to false when hit and set visibility to true when no longer hit. To improve: transparency fading in and out.
  (bind _outhits (Collision|MultiLineTraceByChannel (Transformation|GetWorldLocation (Variables|/Script/HoopSnake.HoopSnakeCharacter|GetFollowCamera _snake)) (Transformation|GetWorldLocation (Variables|/Script/HoopSnake.HoopSnakeCharacter|GetCameraBoom _snake)) "TraceTypeQuery1" false 0 "None"))
  (Utilities|Array|Clear (Variables|Default|GetHitObstacles))
  (for _array_element _outhits
    (bind _asbp_obstacle (Utilities|Casting|CastToBP_Obstacle (.HitActor (Collision|BreakHitResult _array_element))))
    (Utilities|Array|AddUnique (Variables|Default|GetHitObstacles) _asbp_obstacle)
    (Utilities|Array|AddUnique (Variables|Default|GetOccludedObstacles) _asbp_obstacle)
    (Rendering|SetVisibility (Variables|/Game/HoopSnake/Blueprints/BP_Obstacle.BP_Obstacle_C|GetStaticMesh _asbp_obstacle) false false))
  (for _array_element_2 (Variables|Default|GetOccludedObstacles)
    (if (not (Utilities|Array|ContainsItem (Variables|Default|GetHitObstacles) _array_element_2))
      (Rendering|SetVisibility (Variables|/Game/HoopSnake/Blueprints/BP_Obstacle.BP_Obstacle_C|GetStaticMesh _array_element_2) true false))))